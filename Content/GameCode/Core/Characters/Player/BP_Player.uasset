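; Player character Blueprint that adds a sprint camera effect on top of its parent class's sprint handling.
; It caches the spring arm's default length on BeginPlay, then a timeline lerps it toward the sprint length on sprint start and reverses on sprint end.
; Right mouse button directly plays a chest push reaction montage.
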(event `self.ReceiveBeginPlay`
  (set `self.DefaultArmLength` (`SpringArmComponent.TargetArmLength` (`self.SpringArmComponent`))))

(event `self.OnSprintStart`
  (`parent.OnSprintStart`)
  (bind (_direction _newtrack_0) (`Timeline|Spring arm sprint timeline` :!label _label)
    (:`Update`
      (set `SpringArmComponent.TargetArmLength` (`KismetMathLibrary.Lerp` (`self.DefaultArmLength`) (`self.SprintArmLength`) _newtrack_0) (`self.SpringArmComponent`)))))

(event `self.OnSprintEnd`
  (`parent.OnSprintEnd`)
  (goto _label :!via `Reverse`))

(event `Key|RightMouseButton`
  (params (Key :type "Key Structure"))
  (:`Pressed`
    (`self.PlayAnimMontage` "/Game/UpperCard/Core/Characters/Animations/RamsterZ/AM_P_ChestPush_Reaction.AM_P_ChestPush_Reaction")))

(fn `UserConstructionScript`)